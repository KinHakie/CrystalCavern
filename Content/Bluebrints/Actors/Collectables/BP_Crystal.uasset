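; Collectable crystal that, when the player overlaps it, animates toward the player and adds one to the player pawn's collected crystal count.
; Overlap stores the starting location, scale and light intensity, then plays a timeline that lerps the crystal to the player's current position while shrinking it and fading its point light.
; When the timeline finishes, it destroys the actor and increments CollectedCrystals on BP_PlayerPawn.
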(event `self.ReceiveActorBeginOverlap`
  (params (OtherActor :type "Actor Object Reference"))
  (`/Game/Bluebrints/Libraries/CC_MarcoLibrarie.IsPlayer` OtherActor
    (:`IsPlayer`
      (`self.StoreStartingValues`)
      (bind (_direction _collectionprogress _light_intensity) (`Timeline|CollectTimeline`)
        (:`Update`
          (`self.MoveToPlayer` _collectionprogress)
          (`self.Scale Crystal` _collectionprogress)
          (`self.Adjust light` _light_intensity))
        (:`Finished`
          (`self.K2_DestroyActor`)
          (bind _asbp_player_pawn (cast `/Game/Bluebrints/PlayerPawn/BP_PlayerPawn` (`GameplayStatics.GetPlayerPawn` 0)))
          (set `/Game/Bluebrints/PlayerPawn/BP_PlayerPawn.CollectedCrystals` (+ (`/Game/Bluebrints/PlayerPawn/BP_PlayerPawn.CollectedCrystals` _asbp_player_pawn) 1) _asbp_player_pawn))))))

(fn `Adjust light`
  (params (Alpha :type "Float (double-precision)"))
  (`LightComponent.SetIntensity` (`self.PointLight`) (`KismetMathLibrary.Lerp` (`self.Intensity`) 0.0 Alpha)))

(fn `MoveToPlayer`
  (params (Alpha :type "Float (double-precision)"))
  (`self.K2_SetActorLocation` (`KismetMathLibrary.VLerp` (`self.StartLocation`) (`self.K2_GetActorLocation` (`GameplayStatics.GetPlayerPawn` 0)) Alpha)))

(fn `Scale Crystal`
  (params (Alpha :type "Float (double-precision)"))
  (`self.SetActorScale3D` (`KismetMathLibrary.VLerp` (`self.StartScale`) (0.0 0.0 0.0) Alpha)))

(fn `StoreStartingValues`
  (set `self.StartLocation` (`self.K2_GetActorLocation`))
  (set `self.StartScale` (`self.GetActorScale3D`))
  (set `self.Intensity` (`LightComponentBase.Intensity` (`self.PointLight`))))

(fn `UserConstructionScript`)