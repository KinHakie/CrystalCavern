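; BP_Cannon is an obstacle actor that fires projectiles repeatedly from BeginPlay.
; After a CannonFireRate delay, it spawns a BP_Projectile at the ProjectileSpawn component's location and rotation, scaled by ProjectileScale.
; A timeline then animates the barrel along its relative Y axis, and its Cannon Fired event loops back to the delay for the next shot.
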(event `self.ReceiveBeginPlay`
  (`KismetSystemLibrary.Delay` (`self.CannonFireRate`) :!label _label)
  (`self.SpawnProjectile`)
  (bind (_direction _cannonbarrellocation) (`Timeline|Timeline_0` :!via `PlayFromStart`)
    (:`Update`
      (`self.MoveCannonBarrel` _cannonbarrellocation))
    (:`CannonFired`
      (goto _label))))

(fn `MoveCannonBarrel`
  (params (CannonBarrelLocation :type "Float (double-precision)"))
  (`SceneComponent.K2_SetRelativeLocation` (`self.Cannon`) (`KismetMathLibrary.MakeVector` 0.0 CannonBarrelLocation) false false))

(fn `SpawnProjectile`
  (bind _projectilespawn (`self.ProjectileSpawn`))
  (`|SpawnActorFromClass` "/Game/Bluebrints/Actors/Projectiles/BP_Projectile.BP_Projectile_C" (`KismetMathLibrary.MakeTransform` (`SceneComponent.K2_GetComponentLocation` _projectilespawn) (`SceneComponent.K2_GetComponentRotation` _projectilespawn) (`KismetMathLibrary.Conv_DoubleToVector` (`self.Projectile Scale`))) "Undefined" "OverrideRootScale" null null))

(fn `UserConstructionScript`)